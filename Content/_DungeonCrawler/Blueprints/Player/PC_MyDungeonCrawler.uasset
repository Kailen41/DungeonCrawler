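; Player controller for the dungeon crawler that steers the controlled pawn toward the mouse cursor while MoveAction is held.
; The input press and release toggle a flag that Tick checks.
; While it is set, Tick traces under the cursor on the Visibility channel and feeds the direction to the hit point into AddMovementInput, with no pathfinding.
; The trace's success result is not checked.
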(event `InputAction|MoveAction`
  (params (Key :type "Key Structure"))
  (:`Pressed`
    (set `self.IsMoveActionEnable?` true))
  (:`Released`
    (set `self.IsMoveActionEnable?` false)))

(event `self.ReceiveTick`
  (params (DeltaSeconds :type "Float (single-precision)"))
  ;[1 0 1] Movement functionality
  (if (`self.IsMoveActionEnable?`)
    (`Pawn.AddMovementInput` (`self.K2_GetPawn`) (`KismetMathLibrary.GetDirectionUnitVector` (`self.K2_GetActorLocation` (`self.K2_GetPawn`)) (`.Location` (`GameplayStatics.BreakHitResult` (`self.GetHitResultUnderCursorByChannel` "TraceTypeQuery1")))) 1.0 false)))

(fn `UserConstructionScript`)